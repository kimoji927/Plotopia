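; Base Blueprint for GAS enemy characters that smoothly turns the enemy to face a target actor.
; RotatetoTarget plays a timeline whose track feeds SetFacingRotation as the blend alpha.
; SetFacingRotation stores the pitch toward the target and quaternion-slerps actor rotation toward a height-flattened look-at, so only yaw follows the target.
; GetTimelineLength exposes the turn duration to callers.
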(event `self.RotateToTarget`
  (params (RotateTarget :type "Actor Object Reference"))
  (bind (_direction _rotatetrack) (`Timeline|RotationTimeline` :!via `PlayFromStart`)
    (:`Update`
      (`self.SetFacingRotation` _rotatetrack RotateTarget))))

(fn `GetTimelineLength`
  (returns (ReturnValue :type "Float (single-precision)"))
  (return (`TimelineComponent.GetTimelineLength` (`self.RotationTimeline`))))

(fn `SetFacingRotation`
  (params (Alpha :type "Float (double-precision)") (RotateTarget :type "Actor Object Reference"))
  (bind (_returnvalue_x _returnvalue_y) (`KismetMathLibrary.BreakVector` (`self.K2_GetActorLocation`)))
  (bind (_returnvalue_x_2 _returnvalue_y_2) (`KismetMathLibrary.BreakVector` (`self.K2_GetActorLocation` (`local.RotateTarget`))))
  (bind (_returnvalue_x_3 _returnvalue_y_3 _returnvalue_z) (`KismetMathLibrary.BreakVector` (`KismetMathLibrary.Normal` (- (`self.K2_GetActorLocation` (`local.RotateTarget`)) (`self.K2_GetActorLocation`)))))
  (`local.RotateTarget`
    (:`then`
      (set `self.Pitch` (`KismetMathLibrary.DegAsin` _returnvalue_z))
      (`self.K2_SetActorRotation` (`KismetMathLibrary.Quat_Rotator` (`KismetMathLibrary.Quat_Slerp` (`KismetMathLibrary.Conv_RotatorToQuaternion` (`self.K2_GetActorRotation`)) (`KismetMathLibrary.Conv_RotatorToQuaternion` (`KismetMathLibrary.FindLookAtRotation` (`KismetMathLibrary.MakeVector` _returnvalue_x _returnvalue_y) (`KismetMathLibrary.MakeVector` _returnvalue_x_2 _returnvalue_y_2))) (`local.Alpha`)))))
    (:`else`)))

(fn `UserConstructionScript`)