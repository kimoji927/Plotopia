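; Game instance for the GAS game that handles network session teardown on errors and on leaving.
; Travel and network error events print the failure type, then share one path that destroys the session for player controller 0.
; LeaveSession opens the Startup level first, then destroys the session; the error paths do not change level.
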(event `self.HandleTravelError`
  (params (FailureType :type "ETravelFailure Enum" :default "NoLevel"))
  (`KismetSystemLibrary.PrintString` (`|GetEnumeratorNameAsString` FailureType) true true (struct :`R` 1.0 :`A` 1.0) 5.0)
  (`DestroySessionCallbackProxy.DestroySession` (`GameplayStatics.GetPlayerController` 0) :!label _label))

(event `self.HandleNetworkError`
  (params (FailureType :type "ENetworkFailure Enum" :default "NetDriverAlreadyExists") (bIsServer :type Boolean))
  (`KismetSystemLibrary.PrintString` (`|GetEnumeratorNameAsString` FailureType) true true (struct :`R` 1.0 :`A` 1.0) 5.0)
  (goto _label))

(event `LeaveSession`
  (`GameplayStatics.OpenLevel` "Startup")
  (`DestroySessionCallbackProxy.DestroySession` (`GameplayStatics.GetPlayerController` 0)))