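; BP_Building2 is a test building actor that feeds wall dimensions into a PCG graph.
; Its Construction Script writes vector parameters to the PCG component's graph instance: four wall offsets at half WallWidth along positive and negative X and Y.
; It also sets the "Povit" parameter's Y from WallThickness.
; The event graph holds only disabled stubs, so the Blueprint has no runtime logic of its own.
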(event EventBeginPlay)

(event Collision|EventActorBeginOverlap
  (params (OtherActor :type Actor%20Object%20Reference)))

(event EventTick
  (params (DeltaSeconds :type Float%20%28single-precision%29)))

(fn ConstructionScript
  (bind _wallwidth (Variables|Default|GetWallWidth))
  (bind _pcg (Variables|Default|GetPCG))
  (bind _returnvalue (/ _wallwidth 2.0))
  (bind _graphinstance (Variables|/Script/PCG.PCGComponent|GetGraphInstance _pcg))
  (bind _returnvalue_2 (* _returnvalue -1.0))
  (Effects|Components|ParticleSystem|SetVectorParameter _graphinstance "WallOffest1" (Math|Vector|MakeVector _returnvalue 0.0 0.0))
  (Effects|Components|ParticleSystem|SetVectorParameter _graphinstance "WallOffest2" (Math|Vector|MakeVector _returnvalue_2 0.0 0.0))
  (Effects|Components|ParticleSystem|SetVectorParameter _graphinstance "WallOffest3" (Math|Vector|MakeVector 0.0 _returnvalue 0.0))
  (Effects|Components|ParticleSystem|SetVectorParameter _graphinstance "WallOffest4" (Math|Vector|MakeVector 0.0 _returnvalue_2 0.0))
  (Effects|Components|ParticleSystem|SetVectorParameter _graphinstance "Povit" (Math|Vector|MakeVector 0.0 (Variables|Default|GetWallThickness) 0.0)))