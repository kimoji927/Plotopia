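; PCG Blueprint element that stacks copies of a floor's points to build the storeys or roof level of a building.
; It copies points and metadata from the "In" pin, offsetting each along its own up vector by BuildingHeight per floor.
; OnlyCopytTheRoof instead produces a single copy at Floors times that height.
; It returns the new point data after the first input, so later inputs are not processed.
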(fn ExecutewithContext
  (params (InContext :type PCG%20Context%20Structure%20%28by%20ref%29) (Input :type PCG%20Data%20Collection%20Structure%20%28by%20ref%29))
  (bind _returnvalue (Data|GetInputsbyPinLabel Input "In")) ; 获取名为 "In" 的输入数据列表
  (for _array_element _returnvalue ; 逐个查看列表里的数据
    (bind _aspcg点数据 (Utilities|Casting|CastToPCGPointData (.Data (PCG|TaggedData|BreakTaggedData _array_element)))) ; 把剥离出来的“数据本体”强制转换成 PCG点数据类型
    (bind _output_get (LocalVariables|SetInPointData _aspcg点数据)) ; 将这些PCG点数据缓存为InPointData
    (bind _returnvalue_2 (Metadata|MutableMetadata _output_get)) ; 获取这个点数据的可变元数据 (Mutable Metadata)
    (LocalVariables|SetInMetaData _returnvalue_2)
    (bind _returnvalue_3 (Game|ConstructObjectfromClass "/Script/PCG.PCGPointData")) ; 新建空的输出点数据
    (bind _output_get_2 (LocalVariables|SetOutPointData _returnvalue_3)) ; 并将这个空的输出点数据缓存下来
    (bind _returnvalue_4 (Metadata|MutableMetadata _output_get_2)) ; 获取这个空的输出点数据的可变元数据
    (LocalVariables|SetOutMetaData _returnvalue_4)
    (PCG|Metadata|AddAttributes (LocalVariables|GetOutMetaData) (LocalVariables|GetInMetaData)) ; 把输入元数据的属性描述补齐到输出元数据
    ;[0.15 0.15 0.15 0.5] 将传入的这个平面上所有点的属性值复制给Out元数据,并沿着Out元数据中Location的Z轴按楼层往上平移Floor-1个BuildingHeight单位长度,再将这些点存入AllPoints
    (for _index (range 0 (select (Variables|Default|GetOnlyCopytTheRoof) 0 (- (Variables|Default|GetFloors) 1)))
      (for _array_element_2 (SpatialData|GetPoints (LocalVariables|GetInPointData))
        (bind _outpoint (PCG|CopyPoint _array_element_2 true (LocalVariables|GetInMetaData) (LocalVariables|GetOutMetaData)))
        (bind _structout (Utilities|Struct|SetmembersinPCGPoint _outpoint (Math|Transform|MakeTransform (+ (.location (.Transform (Utilities|Struct|BreakPCGPoint _outpoint))) (* (Math|Vector|GetUpVector (.rotation (.Transform (Utilities|Struct|BreakPCGPoint _outpoint)))) (* (Variables|Default|GetBuildingHeight) (select (Variables|Default|GetOnlyCopytTheRoof) (Variables|Default|GetFloors) _index)))) (.rotation (.Transform (Utilities|Struct|BreakPCGPoint _outpoint))) (.scale (.Transform (Utilities|Struct|BreakPCGPoint _outpoint))))))
        (Utilities|Array|Add (LocalVariables|GetAllPoints) _structout)))
    (SpatialData|SetPoints (LocalVariables|GetOutPointData) (LocalVariables|GetAllPoints)) ; 将AllPoints的点设置给输出点数据
    (return (Utilities|Struct|MakePCGDataCollection (Utilities|Array|MakeArray (Utilities|Struct|MakePCGTaggedData (LocalVariables|GetOutPointData) 0 "None"))))))