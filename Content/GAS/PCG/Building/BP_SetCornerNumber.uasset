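; Custom PCG Blueprint node for building generation that tags points with a CornerNumber attribute classifying their corner configuration.
; ExecuteWithContext caches point locations and rotations, then probes for neighbours one InteriorSampleSpacing along each point's forward axis and at half-spacing diagonals.
; HasCurrentPoint does these tolerance-based linear searches, sorting point indices into eight arrays.
; PointLoopBody copies each point and writes its number by index, or zero if unmatched.
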(fn ExecutewithContext
  (params (InContext :type PCG%20Context%20Structure%20%28by%20ref%29) (Input :type PCG%20Data%20Collection%20Structure%20%28by%20ref%29))
  (bind _allpointslocation (LocalVariables|GetAllPointsLocation))
  (bind _interiorsamplespacing (Variables|Default|GetInteriorSampleSpacing))
  (bind _interiorsamplespacing_2 (Variables|Default|GetInteriorSampleSpacing))
  (bind _returnvalue (/ _interiorsamplespacing_2 2.0))
  ;[0.15 0.15 0.15 0.5] 先将所有传入点的位置和旋转缓存起来
  (bind _returnvalue_2 (Data|GetInputsbyPinLabel Input "In"))
  (for _array_element _returnvalue_2
    (bind _aspcg点数据 (Utilities|Casting|CastToPCGPointData (.Data (PCG|TaggedData|BreakTaggedData _array_element))))
    (bind _output_get (LocalVariables|SetInPointData _aspcg点数据))
    (for _array_element_2 (SpatialData|GetPoints _output_get)
      (Utilities|Array|Add (LocalVariables|GetAllPointsLocation) (.location (.Transform (Utilities|Struct|BreakPCGPoint _array_element_2))))
      (Utilities|Array|Add (LocalVariables|GetAllPointsRotation) (.rotation (.Transform (Utilities|Struct|BreakPCGPoint _array_element_2)))))
    (for (_array_element_3 _array_index) (LocalVariables|GetAllPointsRotation)
      (LocalVariables|SetCurrentPointRotation _array_element_3)
      (LocalVariables|SetCurrentPointLocation (Utilities|Array|Get(acopy) (LocalVariables|GetAllPointsLocation) _array_index))
      (LocalVariables|SetCurrentPointIndex _array_index)
      ;[0.15 0.15 0.15 0.5] 判断当前点的转角编号并存入对应的数组中
      (if (and (not (CallFunction|HasCurrentPoint _allpointslocation (+ (* (Math|Vector|GetForwardVector (LocalVariables|GetCurrentPointRotation)) _interiorsamplespacing -1.0) (LocalVariables|GetCurrentPointLocation)) 1.0)) (not (CallFunction|HasCurrentPoint _allpointslocation (+ (LocalVariables|GetCurrentPointLocation) (* (Math|Vector|GetForwardVector (LocalVariables|GetCurrentPointRotation)) _interiorsamplespacing)) 1.0)))
        (if (and (CallFunction|HasCurrentPoint _allpointslocation (+ (LocalVariables|GetCurrentPointLocation) (* (Math|Vector|GetForwardVector (LocalVariables|GetCurrentPointRotation)) _returnvalue -1.0) (* (Math|Vector|GetRightVector (LocalVariables|GetCurrentPointRotation)) _returnvalue -1.0)) 1.0) (CallFunction|HasCurrentPoint _allpointslocation (+ (LocalVariables|GetCurrentPointLocation) (* (Math|Vector|GetForwardVector (LocalVariables|GetCurrentPointRotation)) _returnvalue) (* (Math|Vector|GetRightVector (LocalVariables|GetCurrentPointRotation)) _returnvalue)) 1.0)) ; 1左上右下有
          (Utilities|Array|Add (Variables|Default|Get1) (LocalVariables|GetCurrentPointIndex))
          (elif (and (CallFunction|HasCurrentPoint _allpointslocation (+ (LocalVariables|GetCurrentPointLocation) (* (Math|Vector|GetForwardVector (LocalVariables|GetCurrentPointRotation)) _returnvalue) (* (Math|Vector|GetRightVector (LocalVariables|GetCurrentPointRotation)) _returnvalue -1.0)) 1.0) (CallFunction|HasCurrentPoint _allpointslocation (+ (LocalVariables|GetCurrentPointLocation) (* (Math|Vector|GetForwardVector (LocalVariables|GetCurrentPointRotation)) _returnvalue -1.0) (* (Math|Vector|GetRightVector (LocalVariables|GetCurrentPointRotation)) _returnvalue)) 1.0)) ; 2右上左下有
            (Utilities|Array|Add (Variables|Default|Get2) (LocalVariables|GetCurrentPointIndex))
            (elif (and (CallFunction|HasCurrentPoint _allpointslocation (+ (LocalVariables|GetCurrentPointLocation) (* (Math|Vector|GetForwardVector (LocalVariables|GetCurrentPointRotation)) _returnvalue) (* (Math|Vector|GetRightVector (LocalVariables|GetCurrentPointRotation)) _returnvalue)) 1.0) (CallFunction|HasCurrentPoint _allpointslocation (+ (LocalVariables|GetCurrentPointLocation) (* (Math|Vector|GetForwardVector (LocalVariables|GetCurrentPointRotation)) _returnvalue -1.0) (* (Math|Vector|GetRightVector (LocalVariables|GetCurrentPointRotation)) _returnvalue)) 1.0)) ; 3左下右下有
              (Utilities|Array|Add (Variables|Default|Get3) (LocalVariables|GetCurrentPointIndex))
              (else
                (Utilities|Array|Add (Variables|Default|Get4) (LocalVariables|GetCurrentPointIndex))))))
        (elif (Math|Boolean|ANDBoolean (not (CallFunction|HasCurrentPoint _allpointslocation (+ (* (Math|Vector|GetForwardVector (LocalVariables|GetCurrentPointRotation)) _interiorsamplespacing -1.0) (LocalVariables|GetCurrentPointLocation)) 1.0)) (CallFunction|HasCurrentPoint _allpointslocation (+ (LocalVariables|GetCurrentPointLocation) (* (Math|Vector|GetForwardVector (LocalVariables|GetCurrentPointRotation)) _interiorsamplespacing)) 1.0) (CallFunction|HasCurrentPoint _allpointslocation (+ (LocalVariables|GetCurrentPointLocation) (* (Math|Vector|GetForwardVector (LocalVariables|GetCurrentPointRotation)) _returnvalue -1.0) (* (Math|Vector|GetRightVector (LocalVariables|GetCurrentPointRotation)) _returnvalue -1.0)) 1.0)) ; 5左无右有左上有
          (Utilities|Array|Add (Variables|Default|Get5) (LocalVariables|GetCurrentPointIndex))
          (elif (Math|Boolean|ANDBoolean (not (CallFunction|HasCurrentPoint _allpointslocation (+ (* (Math|Vector|GetForwardVector (LocalVariables|GetCurrentPointRotation)) _interiorsamplespacing -1.0) (LocalVariables|GetCurrentPointLocation)) 1.0)) (CallFunction|HasCurrentPoint _allpointslocation (+ (LocalVariables|GetCurrentPointLocation) (* (Math|Vector|GetForwardVector (LocalVariables|GetCurrentPointRotation)) _interiorsamplespacing)) 1.0) (CallFunction|HasCurrentPoint _allpointslocation (+ (LocalVariables|GetCurrentPointLocation) (* (Math|Vector|GetForwardVector (LocalVariables|GetCurrentPointRotation)) _returnvalue -1.0) (* (Math|Vector|GetRightVector (LocalVariables|GetCurrentPointRotation)) _returnvalue)) 1.0)) ; 6左无右有左下有
            (Utilities|Array|Add (Variables|Default|Get6) (LocalVariables|GetCurrentPointIndex))
            (elif (Math|Boolean|ANDBoolean (CallFunction|HasCurrentPoint _allpointslocation (+ (* (Math|Vector|GetForwardVector (LocalVariables|GetCurrentPointRotation)) _interiorsamplespacing -1.0) (LocalVariables|GetCurrentPointLocation)) 1.0) (not (CallFunction|HasCurrentPoint _allpointslocation (+ (LocalVariables|GetCurrentPointLocation) (* (Math|Vector|GetForwardVector (LocalVariables|GetCurrentPointRotation)) _interiorsamplespacing)) 1.0)) (CallFunction|HasCurrentPoint _allpointslocation (+ (LocalVariables|GetCurrentPointLocation) (* (Math|Vector|GetForwardVector (LocalVariables|GetCurrentPointRotation)) _returnvalue) (* (Math|Vector|GetRightVector (LocalVariables|GetCurrentPointRotation)) _returnvalue -1.0)) 1.0)) ; 7左有右无右上有
              (Utilities|Array|Add (Variables|Default|Get7) (LocalVariables|GetCurrentPointIndex))
              (elif (Math|Boolean|ANDBoolean (CallFunction|HasCurrentPoint _allpointslocation (+ (* (Math|Vector|GetForwardVector (LocalVariables|GetCurrentPointRotation)) _interiorsamplespacing -1.0) (LocalVariables|GetCurrentPointLocation)) 1.0) (not (CallFunction|HasCurrentPoint _allpointslocation (+ (LocalVariables|GetCurrentPointLocation) (* (Math|Vector|GetForwardVector (LocalVariables|GetCurrentPointRotation)) _interiorsamplespacing)) 1.0)) (CallFunction|HasCurrentPoint _allpointslocation (+ (LocalVariables|GetCurrentPointLocation) (* (Math|Vector|GetForwardVector (LocalVariables|GetCurrentPointRotation)) _returnvalue) (* (Math|Vector|GetRightVector (LocalVariables|GetCurrentPointRotation)) _returnvalue)) 1.0)) ; 8左有右无右下有
                (Utilities|Array|Add (Variables|Default|Get8) (LocalVariables|GetCurrentPointIndex))))))))
    (bind _outdata (PCG|FlowControl|PointLoop InContext (LocalVariables|GetInPointData) 0))
    (return (Utilities|Struct|MakePCGDataCollection (Utilities|Array|MakeArray (Utilities|Struct|MakePCGTaggedData _outdata 0 "None"))))))

(fn HasCurrentPoint
  (params (AllPointsLocation :type Array%20of%20Vectors) (ComparePoint :type Vector) (Tolerance :type Float%20%28double-precision%29))
  (bind _array_element (Utilities|Array|ForEachLoopwithBreak AllPointsLocation :!label _label)
    (:LoopBody
      (if (<= (Math|Vector|VectorLength (- _array_element ComparePoint)) Tolerance)
        (LocalVariables|SetIsHasPoint true)
        (goto _label Break)))
    (:Completed
      (return (LocalVariables|GetIsHasPoint)))))

(fn PointLoopBody
  (params (InContext :type PCG%20Context%20Structure%20%28by%20ref%29) (InData :type PCG%20Point%20Data%20Object%20Reference) (InPoint :type PCG%20Point%20Structure%20%28by%20ref%29) (OutMetadata :type PCG%20Metadata%20Object%20Reference) (Iteration :type Integer64))
  (bind _returnvalue (Math|Conversions|ToInteger(Byte) Iteration))
  ;[0.15 0.15 0.15 0.5] 按照点索引的顺序依次设置点的转角编号
  (bind _returnvalue_2 (Metadata|MutableMetadata InData))
  (bind _outpoint (PCG|CopyPoint InPoint true _returnvalue_2 OutMetadata))
  (Class|PCGMetadataAccessorHelpers|SetInteger64Attribute _outpoint OutMetadata "CornerNumber" (select (Utilities|Array|ContainsItem (Variables|Default|Get1) _returnvalue) 1 (select (Utilities|Array|ContainsItem (Variables|Default|Get2) _returnvalue) 2 (select (Utilities|Array|ContainsItem (Variables|Default|Get3) _returnvalue) 3 (select (Utilities|Array|ContainsItem (Variables|Default|Get4) _returnvalue) 4 (select (Utilities|Array|ContainsItem (Variables|Default|Get5) _returnvalue) 5 (select (Utilities|Array|ContainsItem (Variables|Default|Get6) _returnvalue) 6 (select (Utilities|Array|ContainsItem (Variables|Default|Get7) _returnvalue) 7 (select (Utilities|Array|ContainsItem (Variables|Default|Get8) _returnvalue) 8 0)))))))))
  (return _outpoint true))