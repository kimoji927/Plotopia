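; Custom PCG Blueprint node for building generation that assigns a mesh to each point by its corner number.
; It reads the MeshSet attribute set (noted as the parapet mesh set) into a map from Corner to Mesh path.
; A point loop copies each point from the In pin and writes the mesh matching its CornerNumber to the Mesh attribute.
; It returns from inside the loop, so only the first In data is output.
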(fn ExecutewithContext
  (params (InContext :type PCG%20Context%20Structure%20%28by%20ref%29) (Input :type PCG%20Data%20Collection%20Structure%20%28by%20ref%29))
  (bind _returnvalue (Data|GetInputsbyPinLabel Input "MeshSet"))
  (for _array_element _returnvalue
    (bind _aspcg属性集 (Utilities|Casting|CastToPCGParamData (.Data (PCG|TaggedData|BreakTaggedData _array_element))))
    (bind _returnvalue_2 (Metadata|MutableMetadata _aspcg属性集))
    (for _index (range 0 (Math|Conversions|ToInteger(Byte) (- (Class|PCGMetadata|GetItemCountforChild _returnvalue_2) 1)))
      (bind _returnvalue_3 (PCG|Metadata|GetInteger64AttributebyMetadataKey (Class|KismetMathLibrary|ToInt64(Integer) _index) _returnvalue_2 "Corner")) ; ParapetMeshSet中的Corner
      (bind _returnvalue_4 (PCG|Metadata|GetSoftObjectPathAttributebyMetadataKey (Class|KismetMathLibrary|ToInt64(Integer) _index) _returnvalue_2 "Mesh")) ; ParapetMeshSet中的Mesh
      (Utilities|Map|Add (Variables|Default|GetMeshSet) _returnvalue_3 _returnvalue_4))
    (bind _returnvalue_5 (Data|GetInputsbyPinLabel Input "In"))
    (for _array_element_2 _returnvalue_5
      (bind _aspcg点数据 (Utilities|Casting|CastToPCGPointData (.Data (PCG|TaggedData|BreakTaggedData _array_element_2))))
      (bind _outdata (PCG|FlowControl|PointLoop InContext _aspcg点数据 0))
      (return (Utilities|Struct|MakePCGDataCollection (Utilities|Array|MakeArray (Utilities|Struct|MakePCGTaggedData _outdata (.Tags (PCG|TaggedData|BreakTaggedData _array_element_2)) (.Pin (PCG|TaggedData|BreakTaggedData _array_element_2)))))))))

(fn PointLoopBody
  (params (InContext :type PCG%20Context%20Structure%20%28by%20ref%29) (InData :type PCG%20Point%20Data%20Object%20Reference) (InPoint :type PCG%20Point%20Structure%20%28by%20ref%29) (OutMetadata :type PCG%20Metadata%20Object%20Reference) (Iteration :type Integer64))
  (bind _returnvalue (Metadata|MutableMetadata InData))
  (bind _outpoint (PCG|CopyPoint InPoint true _returnvalue OutMetadata))
  (bind _returnvalue_2 (Class|PCGMetadataAccessorHelpers|GetInteger64Attribute _outpoint OutMetadata "CornerNumber"))
  (if (.ReturnValue (Utilities|Map|Find (Variables|Default|GetMeshSet) _returnvalue_2))
    (Class|PCGMetadataAccessorHelpers|SetSoftObjectPathAttribute _outpoint OutMetadata "Mesh" (.Value (Utilities|Map|Find (Variables|Default|GetMeshSet) _returnvalue_2))))
  (return _outpoint true))