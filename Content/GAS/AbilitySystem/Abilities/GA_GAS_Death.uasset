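; Gameplay ability that handles character death and respawn in GAS.
; It plays the death montage while applying GE_Death to tag the owner dead.
; When the montage ends, non-respawning enemies are hidden and given a short lifespan, while all other characters respawn.
; Respawn removes the Dead-tag effect, sends an EndAttack event, resets attributes and moves to a player start on authority, then calls HandleRespawn and ends the ability.
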(event `self.K2_ActivateAbility`
  (bind _returnvalue (`self.GetAbilitySystemComponentFromActorInfo`))
  (bind _returnvalue_2 (`self.GetAvatarActorFromActorInfo`))
  (`AbilityTask_PlayMontageAndWait.CreatePlayMontageAndWaitProxy` "None" (`self.DeathMontage`)
    (:`then`
      ; 贴上死亡标签
      (`AbilitySystemComponent.BP_ApplyGameplayEffectSpecToSelf` _returnvalue (`AbilitySystemComponent.MakeOutgoingSpec` :`self` _returnvalue :`GameplayEffectClass` "/Game/GAS/AbilitySystem/GameplayEffects/GE_Death.GE_Death_C" :`Level` 1.0)))
    (:`OnCompleted`
      (bind _asbp_gas_enemy_base (cast `/Game/GAS/Characters/EnemyCharacters/BP_GAS_EnemyBase` (`self.GetAvatarActorFromActorInfo`) :!label _label)
        (:`then`
          (if (`/Game/GAS/Characters/EnemyCharacters/BP_GAS_EnemyBase.ShouldRespawn` _asbp_gas_enemy_base)
            (`self.RespawnCharacter`)
            (else
              (`Actor.SetLifeSpan` _returnvalue_2 1.0)
              (`Actor.SetActorHiddenInGame` _returnvalue_2 true))))
        (:`CastFailed`
          (`self.RespawnCharacter`))))
    (:`OnInterrupted`
      (goto _label))
    (:`OnCancelled`
      (goto _label))))

(event `RespawnCharacter`
  (`|ExecutionSequence`
    (:`then_0`
      ; 移除死亡标签
      (`self.BP_RemoveGameplayEffectFromOwnerWithGrantedTags` (struct :`GameplayTags` (struct :`(TagName` "GASTags.Status.Dead"))) 1)
      (`AbilitySystemBlueprintLibrary.SendGameplayEventToActor` (`self.GetAvatarActorFromActorInfo`) (struct :`TagName` "GASTags.GASEvents.Enemy.EndAttack")))
    (:`then_1`
      (bind _asgas_base_character (cast `GAS_BaseCharacter` (`self.GetAvatarActorFromActorInfo`)))
      (set `self.GAS Base Character` _asgas_base_character))
    (:`then_2`
      (`self.K2_HasAuthority`
        (:`True`
          (`|ExecutionSequence`
            (:`then_0`
              ; 重置属性
              (bind _gas_base_character (`self.GAS Base Character`)
                (:`then`
                  (`GAS_BaseCharacter.ResetAttributes` _gas_base_character))
                (:`else`)))
            (:`then_1`
              ; 重新设置Actor位置
              (bind _gas_base_character_2 (`self.GAS Base Character`)
                (:`then`
                  (`Actor.K2_SetActorLocation` (`self.GAS Base Character`) (`Actor.K2_GetActorLocation` (`GameModeBase.K2_FindPlayerStart` (`GameplayStatics.GetGameMode`) (`Pawn.GetController` _gas_base_character_2) "")) false false))
                (:`else`)))))))
    (:`then_3`
      (bind _gas_base_character_3 (`self.GAS Base Character`)
        (:`then`
          (`GAS_BaseCharacter.HandleRespawn` _gas_base_character_3))
        (:`else`)))
    (:`then_4`
      (`self.K2_EndAbility`))))