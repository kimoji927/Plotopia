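; Passive-style Gameplay Ability that watches an attribute, health by its name, and triggers death when it reaches zero.
; On activation it starts an async attribute-change listener on the owner's Ability System Component and stores the task.
; Each change optionally prints the new value for debugging and, at zero or below, activates abilities tagged GASTags.GASAbilities.Death, allowing remote activation.
; Ending the ability ends the stored task.
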(event `self.K2_ActivateAbility`
  (bind (_asynctaskproxy _attribute _newvalue) (`GAS_AttributeChangeTask.ListenForAttributeChange` (`self.GetAbilitySystemComponentFromActorInfo`) (struct :`AttributeName` "Health" :`Attribute` "/Script/GAS.GAS_AttributeSet:Health" :`AttributeOwner` "/Script/CoreUObject.Class'/Script/GAS.GAS_AttributeSet'"))
    (:`then`
      (set `self.AttributeChangeTask` _asynctaskproxy))
    (:`OnAttributeChanged`
      (`self.bDrawDebugs`
        (:`then`
          (`KismetSystemLibrary.PrintString` (`KismetStringLibrary.Conv_DoubleToString` _newvalue)))
        (:`else`
          _))
      (if (<= _newvalue 0.0)
        (`AbilitySystemComponent.TryActivateAbilitiesByTag` (`self.GetAbilitySystemComponentFromActorInfo`) (`BlueprintGameplayTagLibrary.MakeGameplayTagContainerFromTag` (`BlueprintGameplayTagLibrary.MakeLiteralGameplayTag` (struct :`TagName` "GASTags.GASAbilities.Death"))) true)))))

(event `self.K2_OnEndAbility`
  (params (bWasCancelled :type Boolean))
  (bind _attributechangetask (`self.AttributeChangeTask`)
    (:`then`
      (`GAS_AttributeChangeTask.EndTask` _attributechangetask))
    (:`else`)))