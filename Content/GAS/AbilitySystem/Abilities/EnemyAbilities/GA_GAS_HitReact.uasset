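; Enemy hit-react gameplay ability that plays a directional montage when the character is hit.
; On activation it listens for the Enemy.HitReact gameplay event and ignores it if the owner has the Dead tag.
; It derives a direction name from the avatar's forward and the vector to the instigator, then jumps the montage to the matching section.
; Optional debug prints show the instigator and direction; the graph never calls EndAbility.
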(event `self.K2_ActivateAbility`
  (bind (_asynctaskproxy _payload) (`AbilityTask_WaitGameplayEvent.WaitGameplayEvent` (struct :`TagName` "GASTags.GASEvents.Enemy.HitReact") null)
    (:`EventReceived`
      (if (not (`GameplayTagAssetInterface.HasMatchingGameplayTag` (`self.GetAbilitySystemComponentFromActorInfo`) (struct :`TagName` "GASTags.Status.Dead")))
        (`self.PrintDebugEventReceived` _payload)
        (`self.CacheHitDirectionVectors` (`.Instigator` (break `GameplayEventData` _payload)))
        (`|ExecutionSequence`
          (:`then_0`
            ; 缓存方向名称并绘制调试
            (set `self.HitDirectionName` (`GAS_BlueprintLibrary.GetDirectionName` (`GAS_BlueprintLibrary.GetHitDirection` (`self.AvatarForward`) (`self.ToInstigator`))))
            (`self.bDrawDebugs`
              (:`then`
                (`KismetSystemLibrary.PrintString` (`KismetStringLibrary.Conv_NameToString` (`self.HitDirectionName`))))
              (:`else`)))
          (:`then_1`
            (`AbilityTask_PlayMontageAndWait.CreatePlayMontageAndWaitProxy` "None" (`self.HitReactMontage`)
              (:`then`
                (`self.MontageJumpToSection` (`self.HitDirectionName`))))))))))

(fn `PrintDebugEventReceived`
  (params (GameplayEventData :type "GameplayEventData Structure (by ref)"))
  (`self.bDrawDebugs`
    (:`then`
      (`KismetSystemLibrary.PrintString` (`KismetStringLibrary.Concat_StrStr` "GA_GAS_HitReact Received Event Form:" (`KismetSystemLibrary.GetDisplayName` (`.Instigator` (break `GameplayEventData` GameplayEventData)))) true true (struct :`R` 1.0 :`A` 1.0)))
    (:`else`)))