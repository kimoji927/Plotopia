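; Enemy ranged attack gameplay ability that plays an attack montage and fires a projectile at the nearest player.
; As the montage starts, the authority searches for the closest player-tagged actor within the enemy's AcceptanceRadius.
; If one is found, it spawns BP_GAS_Projectile from the muzzle socket aimed at it and immediately sends the EndAttack gameplay event to itself.
; The ability ends when the montage completes, is interrupted or is cancelled.
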(event `self.K2_ActivateAbility`
  (bind _returnvalue (`self.GetAvatarActorFromActorInfo`))
  (bind _returnvalue_location (`KismetMathLibrary.BreakTransform` (`SceneComponent.GetSocketTransform` (`self.GetOwningComponentFromActorInfo`) "Muzzle_Front_XForward" "RTS_World")))
  (`AbilityTask_PlayMontageAndWait.CreatePlayMontageAndWaitProxy` "None" "/Game/GAS/Characters/EnemyCharacters/Animation/AM_Attack_Ranged.AM_Attack_Ranged" 1.0 "None" false
    (:`then`
      (`self.K2_HasAuthority`
        (:`True`
          (bind _returnvalue_2 (`GAS_BlueprintLibrary.FindClosestActorWithTag` _returnvalue (`Actor.K2_GetActorLocation` _returnvalue) (`self.PlayerTag`) (`GAS_EnemyCharacter.AcceptanceRadius` (cast `GAS_EnemyCharacter` _returnvalue :!pure true))))
          (`/Engine/EditorBlueprintResources/StandardMacros.IsValid` (break `ClosestActorWithTagResult` _returnvalue_2)
            (:`Is Valid`
              (`|SpawnActorFromClass` "/Game/GAS/GameObjects/BP_GAS_Projectile.BP_GAS_Projectile_C" (`KismetMathLibrary.MakeTransform` _returnvalue_location (`KismetMathLibrary.FindLookAtRotation` _returnvalue_location (`Actor.K2_GetActorLocation` (break `ClosestActorWithTagResult` _returnvalue_2)))) "Undefined" "MultiplyWithRoot" (`self.GetAvatarActorFromActorInfo`) 5.0 null)
              (`AbilitySystemBlueprintLibrary.SendGameplayEventToActor` (`self.GetAvatarActorFromActorInfo`) (struct :`TagName` "GASTags.GASEvents.Enemy.EndAttack")))))))
    (:`OnCompleted`
      (`self.K2_EndAbility` :!label _label))
    (:`OnInterrupted`
      (goto _label))
    (:`OnCancelled`
      (goto _label))))