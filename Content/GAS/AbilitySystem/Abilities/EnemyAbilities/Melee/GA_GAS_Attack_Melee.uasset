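; Gameplay Ability that runs an enemy's melee attack against the player.
; It plays a random attack montage and ends when that completes, is interrupted or is cancelled.
; In parallel, it waits for one MeleeTraceHit gameplay event and sends fixed SetByCaller melee damage with impact particles to the hit target.
; It sends EndAttack to the avatar on ability end, or on activation if already dead, skipping the attack.
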(event `self.K2_ActivateAbility`
  (if (`GameplayTagAssetInterface.HasMatchingGameplayTag` (`self.GetAbilitySystemComponentFromActorInfo`) (struct :`TagName` "GASTags.Status.Dead"))
    (`AbilitySystemBlueprintLibrary.SendGameplayEventToActor` (`self.GetAvatarActorFromActorInfo`) (struct :`TagName` "GASTags.GASEvents.Enemy.EndAttack"))
    (else
      (`|ExecutionSequence`
        (:`then_0`
          ; 播放攻击蒙太奇动画
          (`AbilityTask_PlayMontageAndWait.CreatePlayMontageAndWaitProxy` "None" (`KismetArrayLibrary.Array_Random` (`self.AttackMontages`))
            (:`OnCompleted`
              _)
            (:`OnInterrupted`
              _)
            (:`OnCancelled`
              _))
          (`self.K2_EndAbility`))
        (:`then_1`
          ; 监听碰撞事件，发送伤害给玩家
          (bind (_asynctaskproxy _payload) (`AbilityTask_WaitGameplayEvent.WaitGameplayEvent` (struct :`TagName` "GASTags.GASEvents.Enemy.MeleeTraceHit") null true)
            (:`EventReceived`
              (`GAS_BlueprintLibrary.SendDamageEventToPlayer` (`.Target` (break `GameplayEventData` _payload)) (`self.Damage Effect`) _payload (`BlueprintGameplayTagLibrary.MakeLiteralGameplayTag` (struct :`TagName` "GASTags.SetByCaller.Melee")) 20.0 (`BlueprintGameplayTagLibrary.MakeLiteralGameplayTag` (struct :`TagName` "GASTags.None")) (`self.ImpactParticles`)))))))))

(event `self.K2_OnEndAbility`
  (params (bWasCancelled :type Boolean))
  (`AbilitySystemBlueprintLibrary.SendGameplayEventToActor` (`self.GetAvatarActorFromActorInfo`) (struct :`TagName` "GASTags.GASEvents.Enemy.EndAttack")))