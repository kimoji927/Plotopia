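; GA_Primary is the player's primary melee attack gameplay ability, alternating between two attack montages via FlipFlop and ending when the montage finishes or is interrupted.
; On activation it applies GE_BlockHitReact to prevent hit reactions during the attack, removing it by granted tag on end.
; A montage-sent gameplay event triggers a hitbox overlap test, sending hit-react events to victims and applying level-scaled GE_PlayerDamage to each.
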(event `self.K2_ActivateAbility`
  (bind _returnvalue (`self.GetAbilitySystemComponentFromActorInfo`))
  (bind _returnvalue_2 (`self.GetAbilitySystemComponentFromActorInfo`))
  (`|ExecutionSequence`
    (:`then_0`
      ; 在玩家出招期间给玩家授予 GASTags.GASAbilities.BlockHitReact 标签，让玩家的攻击动画不会被敌人的攻击打断（免受击硬直）
      (`AbilitySystemComponent.BP_ApplyGameplayEffectSpecToSelf` _returnvalue (`AbilitySystemComponent.MakeOutgoingSpec` :`self` _returnvalue :`GameplayEffectClass` "/Game/GAS/AbilitySystem/GameplayEffects/Player/GE_BlockHitReact.GE_BlockHitReact_C" :`Level` 1.0)))
    (:`then_1`
      ; 播放攻击蒙太奇,蒙太奇里挂了 AN_SendEventToActor 通知
      (`/Engine/EditorBlueprintResources/StandardMacros.FlipFlop`
        (:`A`
          (`AbilityTask_PlayMontageAndWait.CreatePlayMontageAndWaitProxy` "None" "/Game/GAS/Characters/PlayerCharacters/Animations/GAS_Primary_A_Montage.GAS_Primary_A_Montage"
            (:`OnCompleted`
              _)
            (:`OnBlendOut`
              _)
            (:`OnInterrupted`
              _)
            (:`OnCancelled`
              _))
          (`self.K2_EndAbility`))
        (:`B`
          (`AbilityTask_PlayMontageAndWait.CreatePlayMontageAndWaitProxy` "None" "/Game/GAS/Characters/PlayerCharacters/Animations/GAS_Primary_B_Montage.GAS_Primary_B_Montage"
            (:`OnCompleted`
              _)
            (:`OnBlendOut`
              _)
            (:`OnInterrupted`
              _)
            (:`OnCancelled`
              _))
          (`self.K2_EndAbility`))))
    (:`then_2`
      ; 监听动画蒙太奇发送的Primary通知
      (`AbilityTask_WaitGameplayEvent.WaitGameplayEvent` (struct :`TagName` "GASTags.GASEvents.Player.Primary") null
        (:`EventReceived`
          (bind _returnvalue_3 (`GAS_BlueprintLibrary.HitBoxOverlapTest` (`self.GetAvatarActorFromActorInfo`) (`self.HitBoxRadius`) (`self.HitBoxForwardOffest`) (`self.HitBoxElevationOffest`) (`self.bDrawDebugs`)))
          ; 接收整个数组，一次性给所有命中者发 Enemy.HitReact 事件
          (`self.SendHitReactEventToActor` _returnvalue_3)
          (for _array_element _returnvalue_3
            ; 对球形检测到的敌人进行属性集中的血量修改
            (`AbilitySystemComponent.BP_ApplyGameplayEffectSpecToTarget` _returnvalue_2 (`AbilitySystemComponent.MakeOutgoingSpec` :`self` _returnvalue_2 :`GameplayEffectClass` "/Game/GAS/AbilitySystem/GameplayEffects/Player/GE_PlayerDamage.GE_PlayerDamage_C" :`Level` (`KismetMathLibrary.Conv_IntToDouble` (`self.GetAbilityLevel`))) (`AbilitySystemBlueprintLibrary.GetAbilitySystemComponent` _array_element))))))))

(event `self.K2_OnEndAbility`
  (params (bWasCancelled :type Boolean))
  ; 技能结束移除GASTags.GASAbilities.BlockHitReact 标签
  (`self.BP_RemoveGameplayEffectFromOwnerWithGrantedTags` (struct :`GameplayTags` (struct :`(TagName` "GASTags.GASAbilities.BlockHitReact")))))