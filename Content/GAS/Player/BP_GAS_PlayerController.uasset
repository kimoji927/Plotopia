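; Player controller from the GAS player folder that opens and closes the in-game menu with the IA_ESC input action.
; The menu widget is created and added to the viewport on first use, then reused by toggling its visibility between Visible and Collapsed.
; Each toggle switches the mouse cursor and input mode, using Game and UI focused on the menu when open and Game Only when closed or at BeginPlay.
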(event `self.ReceiveBeginPlay`
  (`WidgetBlueprintLibrary.SetInputMode_GameOnly` self))

(event `EnhancedInput|/Game/GAS/Input/GameMenuActions/IA_ESC`
  (params (ActionValue :type Boolean) (ElapsedSeconds :type "Float (double-precision)") (TriggeredSeconds :type "Float (double-precision)") (InputAction :type "InputAction Object Reference" :default "/Game/GAS/Input/GameMenuActions/IA_ESC.IA_ESC"))
  (:`Started`
    (`self.Toggle_GameMenu`)))

(fn `FocusGame`
  (set `self.bShowMouseCursor` false)
  (`WidgetBlueprintLibrary.SetInputMode_GameOnly` self))

(fn `FocusWidget`
  (set `self.bShowMouseCursor` true)
  (`WidgetBlueprintLibrary.SetInputMode_GameAndUIEx` self (`self.WBP_GameMenu`)))

(fn `Toggle_GameMenu`
  (bind _wbp_gamemenu (`self.WBP_GameMenu`))
  (`self.WBP_GameMenu`
    (:`then`
      (if (`Widget.IsVisible` (`self.WBP_GameMenu`))
        (`Widget.SetVisibility` _wbp_gamemenu "Collapsed")
        (`self.FocusGame`)
        (else
          (`Widget.SetVisibility` _wbp_gamemenu "Visible")
          (`self.FocusWidget` :!label _label))))
    (:`else`
      (bind _returnvalue (`|CreateWidget` "/Game/GAS/UI/Startup/WBP_GameMenu.WBP_GameMenu_C" self))
      (bind _output_get (set `self.WBP_GameMenu` _returnvalue))
      (`UserWidget.AddToViewport` _output_get 0)
      (goto _label))))

(fn `UserConstructionScript`)